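; BP_Collectible is a coin pickup for the platforming character.
; When its sphere overlaps BP_PlatformingCharacter, it increments that character's CollectedCoins, prints the new count and destroys itself.
; If the count equals the character's MaxCoins, it also pauses the game and shows the WBP_Gameover widget on the player screen.
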(event OnComponentBeginOverlap(Sphere)
  (params (OverlappedComponent :type Primitive%20Component%20Object%20Reference) (OtherActor :type Actor%20Object%20Reference) (OtherComp :type Primitive%20Component%20Object%20Reference) (OtherBodyIndex :type Integer) (bFromSweep :type Boolean) (SweepResult :type Hit%20Result%20Structure%20%28by%20ref%29))
  (bind _asbp_platforming_character (Utilities|Casting|CastToBP_PlatformingCharacter OtherActor))
  (bind _result (Math|Integer|IncrementInt (Variables|/Game/Variant_Platforming/Blueprints/BP_PlatformingCharacter.BP_PlatformingCharacter_C|GetCollectedCoins _asbp_platforming_character))
    (:%20%20
      (Development|PrintString (Utilities|String|ToString(Integer) _result))
      (if (== _result (Variables|/Game/Variant_Platforming/Blueprints/BP_PlatformingCharacter.BP_PlatformingCharacter_C|GetMaxCoins _asbp_platforming_character))
        (Game|SetGamePaused true)
        (Actor|DestroyActor)
        (bind _returnvalue (UserInterface|CreateWidget "/Game/Assets/WBP_Gameover.WBP_Gameover_C"))
        (UserInterface|Viewport|AddtoPlayerScreen _returnvalue)
        (else
          (Actor|DestroyActor))))))

(event EventBeginPlay)

(event Collision|EventActorBeginOverlap
  (params (OtherActor :type Actor%20Object%20Reference)))

(event EventTick
  (params (DeltaSeconds :type Float%20%28single-precision%29)))

(fn ConstructionScript)